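; Spline-driven pipe actor that builds itself in the construction script from the points of its spline.
; Each segment becomes a spline mesh following the point tangents, with a dynamic material whose V tiling scales with the straight-line distance between its points.
; An HISM places connection pieces at the points: one at each end, the last flipped, and an opposed pair at interior joints.
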(fn `UserConstructionScript`
  (locals (PointCurrent :type Integer) (PointTransform :type "Transform Structure") (GapConst :type "Float (double-precision)" :default 0.0))
  (bind _pointcurrent (`local.PointCurrent`))
  (bind (_returnvalue_inputkey _returnvalue_position _returnvalue_arrivetangent _returnvalue_leavetangent _returnvalue_rotation) (break `SplinePoint` (`SplineComponent.GetSplinePointAt` (`self.Spline`) (`local.PointCurrent`) "Local")))
  (bind (_returnvalue_inputkey_2 _returnvalue_position_2 _returnvalue_arrivetangent_2) (break `SplinePoint` (`SplineComponent.GetSplinePointAt` (`self.Spline`) (+ (`local.PointCurrent`) 1) "Local")))
  (for _index (range (`SplineComponent.GetNumberOfSplinePoints` (`self.Spline`)))
    (set `local.PointCurrent` _index)
    (if (not (== (`local.PointCurrent`) (- (`SplineComponent.GetNumberOfSplinePoints` (`self.Spline`)) 1)))
      (bind _returnvalue (`AddComponent|NODE_AddSplineMeshComponent-0`))
      (bind _returnvalue_2 (`PrimitiveComponent.CreateDynamicMaterialInstance` _returnvalue 0 (`PrimitiveComponent.GetMaterial` _returnvalue 0) "None"))
      (`MaterialInstanceDynamic.SetScalarParameterValue` _returnvalue_2 "UVTilingV" (/ (`KismetMathLibrary.VSize` (- _returnvalue_position _returnvalue_position_2)) 200.0))
      (`SplineMeshComponent.SetStartAndEnd` _returnvalue _returnvalue_position _returnvalue_leavetangent _returnvalue_position_2 _returnvalue_arrivetangent_2 false))
    (set `local.PointTransform` (`KismetMathLibrary.MakeTransform` _returnvalue_position (`KismetMathLibrary.ComposeRotators` (select `bool` (== (- (`SplineComponent.GetNumberOfSplinePoints` (`self.Spline`)) 1) (`local.PointCurrent`)) :`true` (struct :`Yaw` 180.0) :!type "Rotator Structure") _returnvalue_rotation)))
    (if (or (== _pointcurrent 0) (== _pointcurrent (- (`SplineComponent.GetNumberOfSplinePoints` (`self.Spline`)) 1)))
      (`InstancedStaticMeshComponent.AddInstance` (`self.HISM_Connection`) (`local.PointTransform`) false)
      (else
        (`InstancedStaticMeshComponent.AddInstance` (`self.HISM_Connection`) (`KismetMathLibrary.MakeTransform` (.location (`local.PointTransform`)) (.rotation (`local.PointTransform`))) false)
        (`InstancedStaticMeshComponent.AddInstance` (`self.HISM_Connection`) (`KismetMathLibrary.MakeTransform` (.location (`local.PointTransform`)) (`KismetMathLibrary.MakeRotator` (.roll (.rotation (`local.PointTransform`))) (+ (.pitch (.rotation (`local.PointTransform`))) 180.0) (.yaw (.rotation (`local.PointTransform`))))) false)))))